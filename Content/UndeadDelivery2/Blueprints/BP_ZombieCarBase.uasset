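; BP_ZombieCarBase is a zombie car actor whose spline-driving and crash logic is present but disconnected.
; Live Tick only prints the direction from the previous forward vector to the current one, then caches it.
; MoveAlongSpline is empty.
; Unwired chains hold distance-step and timeline movement along AssignedSpline, a physics impulse, and a stop-and-smoke crash with delayed destruction on hitting another car or the player.
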(event `self.ReceiveTick`
  (params (DeltaSeconds :type "Float (single-precision)"))
  (`KismetSystemLibrary.PrintString` (`KismetStringLibrary.Conv_VectorToString` (`KismetMathLibrary.GetDirectionUnitVector` (`self.LastForward`) (`self.GetActorForwardVector`))))
  (set `self.LastForward` (`self.GetActorForwardVector`)))

(event `MoveAlongSpline`)

(event `CustomEvent_0`
  (`self.K2_DestroyActor`))

(fn `UserConstructionScript`)