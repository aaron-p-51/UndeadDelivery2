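; BP_LocationMarker is a marker actor that displays one of its own world coordinates as text.
; The Construction Script sets its TextRender to the actor's X or Y location, chosen by UseX and divided by 100 to convert centimeters to meters.
; The event graph has no active logic, only an unconnected copy that multiplies by 100 instead.
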(event `self.ReceiveBeginPlay`)

(fn `UserConstructionScript`
  (bind (_returnvalue_x _returnvalue_y) (`KismetMathLibrary.BreakVector` (`self.K2_GetActorLocation`)))
  (if (`self.UseX`)
    (`TextRenderComponent.K2_SetText` (`self.TextRender`) (`KismetTextLibrary.Conv_DoubleToText` (/ _returnvalue_x 100.0) "HalfToEven"))
    (else
      (`TextRenderComponent.K2_SetText` (`self.TextRender`) (`KismetTextLibrary.Conv_DoubleToText` (/ _returnvalue_y 100.0) "HalfToEven")))))