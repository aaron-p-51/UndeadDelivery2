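; BP_ZombieCarSpawner periodically triggers vehicle spawns on zombie car paths.
; On BeginPlay, the authority gathers every BP_ZombieCarPath_Old actor and starts a looping timer at SpawnRate.
; Each tick of that timer picks random paths until it finds an unused one, then calls its SpawnVehicle with a random float.
; A UsedPaths set prevents repeats and clears once every path has been used.
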(event `self.ReceiveBeginPlay`
  (`/Engine/EditorBlueprintResources/ActorMacros.Switch Has Authority`
    (:`Authority`
      (bind _outactors (`GameplayStatics.GetAllActorsOfClass` "/Game/UndeadDelivery2/Blueprints/Old/BP_ZombieCarPath_Old.BP_ZombieCarPath_Old_C"))
      (set `self.ZombieCarPath` _outactors)
      (`KismetSystemLibrary.K2_SetTimerDelegate` (delegate `CustomEvent_0`) (`self.SpawnRate`) true))))

(event `CustomEvent_0`
  (`self.SpawnNewCar`))

(fn `SpawnNewCar`
  (locals (FoundPath :type Boolean) (PossiblePath :type "/Game/UndeadDelivery2/Blueprints/Old/BP_ZombieCarPath_Old Object Reference"))
  (bind _possiblepath (`local.PossiblePath`))
  (set `local.FoundPath` false)
  (bind _result (`BlueprintSetLibrary.Set_ToArray` (`self.UsedPaths`)))
  (if (== (`KismetArrayLibrary.Array_Length` _result) (`KismetArrayLibrary.Array_Length` (`self.ZombieCarPath`)))
    (`BlueprintSetLibrary.Set_Clear` (`self.UsedPaths`)))
  (while (not (`local.FoundPath`))
    (bind _output_get (set `local.PossiblePath` (`|GetArrayItem` (`self.ZombieCarPath`) (`KismetMathLibrary.RandomIntegerInRange` 0 (- (`KismetArrayLibrary.Array_Length` (`self.ZombieCarPath`)) 1)))))
    (if (not (`BlueprintSetLibrary.Set_Contains` (`self.UsedPaths`) _output_get))
      (`BlueprintSetLibrary.Set_Add` (`self.UsedPaths`) _possiblepath)
      (`/Game/UndeadDelivery2/Blueprints/Old/BP_ZombieCarPath_Old.SpawnVehicle` _possiblepath (`KismetMathLibrary.RandomFloatInRange` 20.0 25.0))
      (return))))

(fn `UserConstructionScript`)