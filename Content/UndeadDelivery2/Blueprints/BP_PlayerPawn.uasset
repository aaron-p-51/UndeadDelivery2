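; BP_PlayerPawn is the player-controlled vehicle pawn for UndeadDelivery2.
; It forwards the MoveForward and MoveRight axes and the Drift action to MovementComponent as acceleration, turning and drift input.
; The driving logic itself lives outside this graph, which does no per-tick work.
; On BeginPlay it hides VehicleMesh without propagating the change to child components.
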(event `InputAction|Drift`
  (params (Key :type "Key Structure"))
  (:`Pressed`
    (`ArcadeVehicleMovementComponentBase.SetDriftInput` (`self.MovementComponent`) true))
  (:`Released`
    (`ArcadeVehicleMovementComponentBase.SetDriftInput` (`self.MovementComponent`) false)))

(event `self.ReceiveBeginPlay`
  (`SceneComponent.SetVisibility` (`self.VehicleMesh`) false false))

(event `InputAxis|MoveForward`
  (params (AxisValue :type "Float (single-precision)"))
  (`ArcadeVehicleMovementComponentBase.SetAccelerationInput` (`self.MovementComponent`) AxisValue))

(event `InputAxis|MoveRight`
  (params (AxisValue :type "Float (single-precision)"))
  (`ArcadeVehicleMovementComponentBase.SetTurningInput` (`self.MovementComponent`) AxisValue))

(fn `UserConstructionScript`)