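; BP_DeliveryLocation is a placed point that keeps one delivery request active at its position in the delivery game.
; On BeginPlay it spawns a BP_DeliveryRequest at its own transform and stores it as the active request.
; A looping five-second timer checks whether that stored request is still valid and spawns a replacement once it is gone.
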(event `self.ReceiveBeginPlay`
  (`self.SetActive`)
  (`KismetSystemLibrary.K2_SetTimerDelegate` (delegate `CustomEvent_0`) 5.0 true))

(event `CustomEvent_0`
  (bind _result (`self.HasActiveDelivery`))
  (if (not _result)
    (`self.SetActive`)))

(event `SetActive`
  (bind _returnvalue (`|SpawnActorFromClass` "/Game/UndeadDelivery2/Blueprints/BP_DeliveryRequest.BP_DeliveryRequest_C" (`self.GetTransform` self) "Undefined" "OverrideRootScale" null null))
  (set `self.ActiveDeliveryRequest` _returnvalue))

(fn `HasActiveDelivery`
  (returns (Result :type Boolean))
  (`/Engine/EditorBlueprintResources/StandardMacros.IsValid` (`self.ActiveDeliveryRequest`)
    (:`Is Valid`
      (return true))
    (:`Is Not Valid`
      (return false))))

(fn `UserConstructionScript`)